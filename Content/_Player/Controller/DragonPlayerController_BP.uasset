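; Player controller for click-to-move that shows the mouse cursor and uses Game and UI input mode.
; ClickAction deprojects the cursor, line traces on Visibility and spawns a GroundClick effect at the hit point.
; It forwards that point as a move order to a separate PlayerAvatarController, printing an error if that is invalid.
; A successful move request calls TrySetTimeTick on the TimerManager.
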(event `self.ReceiveBeginPlay`
  (set `self.bShowMouseCursor` true)
  (`WidgetBlueprintLibrary.SetInputMode_GameAndUIEx` self null "LockInFullscreen"))

(event `self.ClickAction`
  (`self.InWorldClick`))

(event `Key|LeftMouseButton`
  (params (Key :type "Key Structure")))

(fn `InWorldClick`
  (locals (ClickLocation :type "Vector Structure" :default (0.0 0.0 0.0)))
  (bind (_worldlocation _worlddirection _returnvalue) (`self.DeprojectMousePositionToWorld`))
  (bind _playeravatarcontroller (`self.PlayerAvatarController`))
  (if _returnvalue
    (bind (_outhit _returnvalue_2) (`KismetSystemLibrary.LineTraceSingle` _worldlocation (+ _worldlocation (* _worlddirection 80000.0)) "TraceTypeQuery1"))
    (if _returnvalue_2
      (bind _output_get (set `local.ClickLocation` (`.ImpactPoint` (`GameplayStatics.BreakHitResult` _outhit))))
      ;[1 1 1] Spawning Click Effect
      (`|SpawnActorFromClass` "/Game/Effects/GroundClick.GroundClick_C" (`KismetMathLibrary.MakeTransform` _output_get) "AlwaysSpawn" "MultiplyWithRoot" null null)
      (`/Engine/EditorBlueprintResources/StandardMacros.IsValid` _playeravatarcontroller
        (:`Is Valid`
          (bind _returnvalue_3 (`BaseAvatarAIController.MoveOrder` _playeravatarcontroller (`local.ClickLocation`)))
          (switch `EPathFollowingRequestResult` _returnvalue_3
            (:`RequestSuccessful`
              (`TimeManager.TrySetTimeTick` (`self.TimerManager`) "Tick"))))
        (:`Is Not Valid`
          (`KismetSystemLibrary.PrintString` "Player avatar is not valid" true true (struct :`R` 1.0 :`B` 0.02448 :`A` 1.0)))))))

(fn `UserConstructionScript`)