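; Raid party enemy avatar that travels along a spline path and carries a Strength value shown by a child actor.
; On BeginPlay it adds the RaidParty gameplay tag and seeds a random small starting strength.
; Point updates and queries for None, Strength and Energy all route to that child actor, while Gold and Temporary Energy queries return zero.
; MoveAlongSpline advances its position by MoveSpeed and DeltaTime without sweeping.
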(event `self.ReceiveBeginPlay`
  (`BlueprintGameplayTagLibrary.AddGameplayTag` (`self.GameplayTags`) (struct :`TagName` "Avatar.RaidParty"))
  (message `/Game/Blueprints/PointSystem/BPI_PointSystemActor.UpdatePoint` (`ChildActorComponent.ChildActor` (`self.StrengthNumber`)) (`KismetMathLibrary.RandomIntegerInRange` 1 3) 0))

(event `/Game/Blueprints/PointSystem/BPI_PointSystemActor.A_UpdatePoint`
  (params (PointType :type "/Game/Blueprints/PointSystem/Enum_PointSystem Enum" :default "NewEnumerator3") (AddValue :type Integer) (SubtractValue :type Integer))
  (switch `/Game/Blueprints/PointSystem/Enum_PointSystem` PointType
    (:`NewEnumerator3`
      _)
    (:`NewEnumerator0`
      _)
    (:`NewEnumerator2`
      _))
  (message `/Game/Blueprints/PointSystem/BPI_PointSystemActor.UpdatePoint` (`ChildActorComponent.ChildActor` (`self.StrengthNumber`)) AddValue SubtractValue))

(event `self.ReceiveTick`
  (params (DeltaSeconds :type "Float (single-precision)")))

(event `self.StartMovement`
  (params (path :type "SplineComponent Object Reference"))
  (`parent.StartMovement` path))

(event `self.MoveAlongSpline`
  (params (DeltaTime :type "Float (single-precision)"))
  (`self.K2_SetActorLocation` (`SplineComponent.GetLocationAtDistanceAlongSpline` (`self.Path`) (`self.DistanceAlongSpline`) "World"))
  (set `self.DistanceAlongSpline` (+ (`self.DistanceAlongSpline`) (* (`self.MoveSpeed`) DeltaTime))))

(fn `A_GetPoint`
  (params (PointType :type "/Game/Blueprints/PointSystem/Enum_PointSystem Enum" :default "NewEnumerator3"))
  (returns (PointValue :type Integer))
  (switch `/Game/Blueprints/PointSystem/Enum_PointSystem` PointType
    (:`NewEnumerator3`
      _)
    (:`NewEnumerator0`
      _)
    (:`NewEnumerator1`
      (return 0))
    (:`NewEnumerator2`
      _)
    (:`NewEnumerator4`
      (return 0)))
  (bind _value (message `/Game/Blueprints/PointSystem/BPI_PointSystemActor.GetPoint` (`ChildActorComponent.ChildActor` (`self.StrengthNumber`))))
  (return _value))

(fn `GetPoint`
  (returns (Value :type Integer))
  (return -1))

(fn `UserConstructionScript`)