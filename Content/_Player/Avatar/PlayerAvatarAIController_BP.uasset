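; AI controller for the player's avatar pawn, handling hoard lookup and sleep energy recovery.
; On possess it finds the Mountain Hoard and registers itself with the DragonPlayerController, using a capped timer retry until that controller is valid.
; While asleep, a looping timer raises the pawn's points by one per tick until they reach a point value read from the hoard; waking clears the timer.
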(event `self.ReceivePossess`
  (params (PossessedPawn :type "Pawn Object Reference"))
  (`self.Timer_Cast to PlayerController`)
  (`self.GetHoard`))

(event `Timer_Cast to PlayerController`
  (if (not (>= (`self.CastToPlayerController_RecursionCount`) (`self.CastToPlayerController_MaxRecursions`)))
    (`/Engine/EditorBlueprintResources/StandardMacros.IsValid` (`GameplayStatics.GetPlayerController` 0)
      (:`Is Valid`
        (`self.Cast To PlayerController`))
      (:`Is Not Valid`
        (`KismetSystemLibrary.K2_SetTimerDelegate` (delegate `Timer_Cast to PlayerController`) 0.5)
        (`/Engine/EditorBlueprintResources/StandardMacros.IncrementInt` (`self.CastToPlayerController_RecursionCount`))))))

(event `Cast To PlayerController`
  (bind _asdragon_player_controller (cast `DragonPlayerController` (`GameplayStatics.GetPlayerController` 0)))
  (set `DragonPlayerController.PlayerAvatarController` self _asdragon_player_controller))

(event `self.EnterSleep`
  (`parent.EnterSleep`)
  (`KismetSystemLibrary.PrintString` "Sleep")
  (bind _returnvalue (`KismetSystemLibrary.K2_SetTimer` null "GetSleepEnergy" 1.0 true))
  (set `self.SleepIterationTimer` _returnvalue))

(event `self.LeaveSleep`
  (`parent.LeaveSleep`)
  (`TimeManager.TrySetTimeTick` (`self.TimerManager`) "LeaveAlwaysTick")
  (`KismetSystemLibrary.K2_ClearAndInvalidateTimerHandle` (`self.SleepIterationTimer`))
  (`KismetSystemLibrary.PrintString` "Waking up"))

(fn `GetHoard`
  (bind _returnvalue (`GameplayStatics.GetActorOfClass` "/Game/Blueprints/StaticEnvironmentPieces/TheMountainHoard.TheMountainHoard_C"))
  (set `self.TheMountainHoard` _returnvalue))

(fn `GetSleepEnergy`
  (bind _pointvalue (`/Game/Blueprints/PointSystem/BPI_PointSystemActor.A_GetPoint` (`self.TheMountainHoard`) "NewEnumerator1"))
  (bind _pointvalue_2 (message `/Game/Blueprints/PointSystem/BPI_PointSystemActor.A_GetPoint` (`self.K2_GetPawn`) "NewEnumerator2"))
  (if (< _pointvalue_2 _pointvalue)
    (message `/Game/Blueprints/PointSystem/BPI_PointSystemActor.A_UpdatePoint` (`self.K2_GetPawn`) "NewEnumerator2" 1 0)))

(fn `UserConstructionScript`)