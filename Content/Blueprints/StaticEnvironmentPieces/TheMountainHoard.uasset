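; The Mountain Hoard is a static environment piece that serves as a gold hoard, tagging itself as a hoard and mountain and seeding starting gold on BeginPlay.
; Point updates and queries are forwarded to a GoldManager child actor, with None treated the same as Gold.
; AlterClickLocation redirects clicks to the HoardPlayerLocation marker, using a vertical trace for surface height and keeping the original click if nothing is hit.
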(event `self.ReceiveBeginPlay`
  (bind _gameplaytags (`self.GameplayTags`))
  (`BlueprintGameplayTagLibrary.AddGameplayTag` _gameplaytags (struct :`TagName` "Avatar.Hoard"))
  (`BlueprintGameplayTagLibrary.AddGameplayTag` _gameplaytags (struct :`TagName` "Mountain"))
  (`/Game/Blueprints/PointSystem/BPI_PointSystemActor.A_UpdatePoint` "NewEnumerator1" 10))

(event `/Game/Blueprints/PointSystem/BPI_PointSystemActor.A_UpdatePoint`
  (params (PointType :type "/Game/Blueprints/PointSystem/Enum_PointSystem Enum" :default "NewEnumerator3") (AddValue :type Integer) (SubtractValue :type Integer))
  (switch `/Game/Blueprints/PointSystem/Enum_PointSystem` PointType
    (:`NewEnumerator3`
      _)
    (:`NewEnumerator1`
      _))
  (message `/Game/Blueprints/PointSystem/BPI_PointSystemActor.UpdatePoint` (`ChildActorComponent.ChildActor` (`self.GoldManager`)) AddValue SubtractValue))

(fn `A_GetPoint`
  (params (PointType :type "/Game/Blueprints/PointSystem/Enum_PointSystem Enum" :default "NewEnumerator3"))
  (returns (PointValue :type Integer))
  (switch `/Game/Blueprints/PointSystem/Enum_PointSystem` PointType
    (:`NewEnumerator3`
      _)
    (:`NewEnumerator1`
      _))
  (bind _value (message `/Game/Blueprints/PointSystem/BPI_PointSystemActor.GetPoint` (`ChildActorComponent.ChildActor` (`self.GoldManager`))))
  (return _value))

(fn `AlterClickLocation`
  (params (ClickLocation :type "Vector Structure"))
  (returns (NewClickLocation :type "Vector Structure"))
  (bind _returnvalue (`SceneComponent.K2_GetComponentLocation` (`self.HoardPlayerLocation`)))
  (bind (_x _y) (`KismetMathLibrary.BreakVector3f` (`SceneComponent.K2_GetComponentLocation` (`self.HoardPlayerLocation`))))
  (bind (_outhit _returnvalue_2) (`KismetSystemLibrary.LineTraceSingle` (+ _returnvalue (0.0 0.0 3000.0)) (- _returnvalue (0.0 0.0 3000.0)) "TraceTypeQuery3"))
  (if _returnvalue_2
    (return (`KismetMathLibrary.MakeVector` _x _y (`.Z` (`KismetMathLibrary.BreakVector3f` (`.ImpactPoint` (`GameplayStatics.BreakHitResult` _outhit))))))
    (else
      (return (`local.ClickLocation`)))))

(fn `GetPoint`
  (returns (Value :type Integer))
  (return 0))

(fn `UserConstructionScript`)