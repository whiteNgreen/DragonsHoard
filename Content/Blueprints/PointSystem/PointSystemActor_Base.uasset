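; Base point-system actor that keeps a points total and shows it on a text render component.
; UpdatePoint adds and subtracts values from the total and refreshes the text, while GetPoint returns it.
; Tick resets the actor's rotation to face the constant world backward direction, keeping the text at a fixed orientation.
; UpdatingEnergy and AUpdatePoint are empty events, and AGetPoint is a stub returning zero.
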(event `self.ReceiveBeginPlay`)

(event `/Game/Blueprints/PointSystem/BPI_PointSystemActor.UpdatePoint`
  (params (AddValue :type Integer) (SubtractValue :type Integer))
  (bind _output_get (set `self.Points` (- (+ (`self.Points`) AddValue) SubtractValue)))
  (`TextRenderComponent.K2_SetText` (`self.TextRender`) (`KismetTextLibrary.Conv_StringToText` (`KismetStringLibrary.Conv_IntToString` _output_get))))

(event `UpdatingEnergy`
  (params (AddToEnergy :type Integer)))

(event `self.ReceiveTick`
  (params (DeltaSeconds :type "Float (single-precision)"))
  (`self.K2_SetActorRotation` (`KismetMathLibrary.MakeRotFromX` (`KismetMathLibrary.Vector_Backward`))))

(event `/Game/Blueprints/PointSystem/BPI_PointSystemActor.A_UpdatePoint`
  (params (PointType :type "/Game/Blueprints/PointSystem/Enum_PointSystem Enum" :default "NewEnumerator3") (AddValue :type Integer) (SubtractValue :type Integer)))

(fn `A_GetPoint`
  (params (PointType :type "/Game/Blueprints/PointSystem/Enum_PointSystem Enum" :default "NewEnumerator3"))
  (returns (PointValue :type Integer))
  (return 0))

(fn `GetPoint`
  (returns (Value :type Integer))
  (return (`self.Points`)))

(fn `UserConstructionScript`)