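; Village actor, filed under Enemies, that tags itself Avatar.Village and holds randomly seeded amounts of two point types.
; On BeginPlay it rolls the starting values, while point updates, transfers and queries are forwarded as messages to the child actor in PointActorComponent.
; VisualDestruction hides that child actor and disables Sphere collision without destroying the village.
; GetPoint is a stub returning zero.
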(event `self.ReceiveBeginPlay`
  (`BlueprintGameplayTagLibrary.AddGameplayTag` (`self.GameplayTags`) (struct :`TagName` "Avatar.Village"))
  (`/Game/Blueprints/PointSystem/BPI_PointSystemActor.A_UpdatePoint` "NewEnumerator0" (`KismetMathLibrary.RandomIntegerInRange` 5 8))
  (`/Game/Blueprints/PointSystem/BPI_PointSystemActor.A_UpdatePoint` "NewEnumerator1" (`KismetMathLibrary.RandomIntegerInRange` 2 4)))

(event `/Game/Blueprints/PointSystem/BPI_PointSystemActor.A_UpdatePoint`
  (params (PointType :type "/Game/Blueprints/PointSystem/Enum_PointSystem Enum" :default "NewEnumerator3") (AddValue :type Integer) (SubtractValue :type Integer))
  (message `/Game/Blueprints/PointSystem/BPI_PointSystemActor.A_UpdatePoint` (`ChildActorComponent.ChildActor` (`self.PointActorComponent`)) PointType AddValue SubtractValue))

(event `/Game/Blueprints/PointSystem/BPI_PointSystemActor.A_TransferPoint`
  (params (PointType :type "/Game/Blueprints/PointSystem/Enum_PointSystem Enum" :default "NewEnumerator3") (From :type "/Game/Blueprints/PointSystem/BPI_PointSystemActor Interface"))
  (message `/Game/Blueprints/PointSystem/BPI_PointSystemActor.A_TransferPoint` (`ChildActorComponent.ChildActor` (`self.PointActorComponent`)) PointType From))

(event `self.VisualDestruction`
  (`self.SetActorHiddenInGame` (`ChildActorComponent.ChildActor` (`self.PointActorComponent`)) true)
  (`PrimitiveComponent.SetCollisionEnabled` (`self.Sphere`) "NoCollision"))

(fn `A_GetPoint`
  (params (PointType :type "/Game/Blueprints/PointSystem/Enum_PointSystem Enum" :default "NewEnumerator3"))
  (returns (PointValue :type Integer))
  (bind _pointvalue (message `/Game/Blueprints/PointSystem/BPI_PointSystemActor.A_GetPoint` (`ChildActorComponent.ChildActor` (`self.PointActorComponent`)) PointType))
  (return _pointvalue))

(fn `GetPoint`
  (returns (Value :type Integer))
  (return 0))

(fn `UserConstructionScript`)