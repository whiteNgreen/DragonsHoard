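; Village path actor that lays a spline-mesh path between an assigned Village and the MountainHordeEntrance_BP in the level.
; Editor events UpdatePath and UpdateSpline pin the spline's first and last points to those two actors, then destroy and rebuild the mesh segments.
; Segment count derives from the mesh's bounding-box length, with tangents clamped to that length.
; The construction script only prints a debug string, so rebuilds rely on those events.
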(event `self.UpdatePath`
  (`self.Construction_MoveSplinepoints` :!label _label)
  (`self.Construction_MakeSplineMesh`))

(event `UpdateSpline`
  (goto _label))

(fn `Construction_MakeSplineMesh`
  (locals (NumberOfInstances :type Integer :default 0) (LoopIndex :type Integer))
  (bind _widthscale (`self.WidthScale`))
  (bind (_min _max) (break `Box` (`StaticMesh.GetBoundingBox` (`self.SplineMesh`))))
  (bind (_arrayindex _arrayelement) (`/Engine/EditorBlueprintResources/StandardMacros.ReverseForEachLoop` (`self.SplineMeshComponents`))
    (:`LoopBody`
      (`ActorComponent.K2_DestroyComponent` _arrayelement))
    (:`Completed`
      (if (`self.bMakeSplineMesh`)
        (set `self.SectionLength` (`KismetMathLibrary.BreakVector3f` (- _max _min)))
        (for _index (range (+ (`KismetMathLibrary.FCeil` (/ (`SplineComponent.GetSplineLength` (`self.PathSpline`)) (+ (`self.SectionLength`) (`self.SectionOffset`)))) 1))
          (set `local.LoopIndex` _index)
          (bind _returnvalue (`AddComponent|NODE_AddSplineMeshComponent-0`))
          (`KismetArrayLibrary.Array_Add` (`self.SplineMeshComponents`) _returnvalue)
          (`StaticMeshComponent.SetStaticMesh` _returnvalue (`self.SplineMesh`))
          (`SplineMeshComponent.SetForwardAxis` _returnvalue "X" true)
          (bind (_start_position _start_tangent _end_position _end_tangent) (`self.Get_TangentPositions` (`local.LoopIndex`)))
          (`SplineMeshComponent.SetStartAndEnd` _returnvalue _start_position _start_tangent _end_position _end_tangent true)
          (`SplineMeshComponent.SetStartScale` _returnvalue (`KismetMathLibrary.MakeVector2D` _widthscale 1.0) true)
          (`SplineMeshComponent.SetEndScale` _returnvalue (`KismetMathLibrary.MakeVector2D` _widthscale 1.0) true))))))

(fn `Construction_MoveSplinepoints`
  (bind _pathspline (`self.PathSpline`))
  (bind _village (`self.Village`))
  (bind _returnvalue (`GameplayStatics.GetActorOfClass` "/Game/_Player/MountainHoard/MountainHordeEntrance_BP.MountainHordeEntrance_BP_C"))
  (`/Engine/EditorBlueprintResources/StandardMacros.IsValid` _returnvalue
    (:`Is Valid`
      (`/Engine/EditorBlueprintResources/StandardMacros.IsValid` _village
        (:`Is Valid`
          (`SplineComponent.SetLocationAtSplinePoint` _pathspline 0 (`self.K2_GetActorLocation` _village) "World" true)
          (`SplineComponent.SetLocationAtSplinePoint` _pathspline (- (`SplineComponent.GetNumberOfSplinePoints` _pathspline) 1) (`self.K2_GetActorLocation` _returnvalue) "World" true))))))

(fn `Get_TangentPositions`
  (params (LoopIndex :type Integer))
  (returns (Start_Position :type "Vector Structure") (Start_Tangent :type "Vector Structure") (End_Position :type "Vector Structure") (End_Tangent :type "Vector Structure"))
  (locals (CoordinateSpace :type "ESplineCoordinateSpace Enum" :default "Local"))
  (bind _pathspline (`self.PathSpline`))
  (bind _pathspline_2 (`self.PathSpline`))
  (bind _coordinatespace (`local.CoordinateSpace`))
  (bind _returnvalue (* (+ LoopIndex 1) (`self.SectionLength`)))
  (bind _returnvalue_2 (* LoopIndex (`self.SectionLength`)))
  (return (`SplineComponent.GetLocationAtDistanceAlongSpline` _pathspline _returnvalue_2 _coordinatespace) (`KismetMathLibrary.ClampVectorSize` (`SplineComponent.GetTangentAtDistanceAlongSpline` _pathspline _returnvalue_2 _coordinatespace) 0.0 (`self.SectionLength`)) (`SplineComponent.GetLocationAtDistanceAlongSpline` _pathspline_2 _returnvalue _coordinatespace) (`KismetMathLibrary.ClampVectorSize` (`SplineComponent.GetTangentAtDistanceAlongSpline` _pathspline_2 _returnvalue _coordinatespace) 0.0 (`self.SectionLength`))))

(fn `UserConstructionScript`
  (`KismetSystemLibrary.PrintString` "Hello"))